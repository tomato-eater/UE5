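; BP_Key is a key pickup that spins in place until the player character collects it.
; A timeline started on BeginPlay drives the yaw of the key mesh.
; When BP_TestChar overlaps the sphere, it saves this key's status, by KeyName, as obtained in the game instance.
; It then calls its SetEventFinished override, which runs the parent logic and destroys the actor.
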(event OnComponentBeginOverlap(Sphere)
  (params (OverlappedComponent :type Primitive%20Component%20Object%20Reference) (OtherActor :type Actor%20Object%20Reference) (OtherComp :type Primitive%20Component%20Object%20Reference) (OtherBodyIndex :type Integer) (bFromSweep :type Boolean) (SweepResult :type Hit%20Result%20Structure%20%28by%20ref%29))
  ;[0.15 0.15 0.15 0.5] 鍵を取得状態にして、自身を消す
  (Utilities|Casting|CastToBP_TestChar OtherActor)
  (Default|SaveKeyStatus (Variables|Default|GetMyGameInstance) (Variables|Default|GetKeyName) "NewEnumerator4")
  (CallFunction|SetEventFinished))

(event EventBeginPlay
  (bind _stm_key (Variables|Default|GetSTM_Key))
  (bind _relativerotation (Variables|/Script/Engine.SceneComponent|GetRelativeRotation _stm_key))
  (bind (_roll _pitch) (Math|Rotator|BreakRotator _relativerotation))
  (if true
    ;[0.15 0.15 0.15 0.5] 回転
    (|CallParentFunction)
    (bind _rotz (Timeline|Rotation Play)
      (:Update
        (Transformation|SetRelativeRotation (Variables|Default|GetSTM_Key) (Math|Rotator|MakeRotator _roll _pitch _rotz) false false)))))

(fn ConstructionScript)

(fn SetEventFinished
  (|CallParentFunction)
  (Actor|DestroyActor))