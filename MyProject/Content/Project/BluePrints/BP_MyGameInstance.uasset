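; Game instance that holds player progress (event and key states, transform, item names) and persists it through BP_MySaveGame.
; It loads the save slot on Init, and each Save function updates its variable then immediately rewrites the slot.
; Status getters fall back to a default enum for missing names.
; Goal_Event clears event and key states in memory and reloads the level, while DeleteSaveData wipes everything including the slot.
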(event Custom|Goal_Event
  (Utilities|Map|Clear (Variables|Default|GetEventStatus))
  (Utilities|Map|Clear (Variables|Default|GetKeyStatus))
  (bind _returnvalue (Game|GetCurrentLevelName true))
  (Game|OpenLevel(byName) (Utilities|String|StringToName _returnvalue)))

(event Custom|ExportSaveData
  (bind _returnvalue (SaveGame|CreateSaveGameObject "/Game/Project/BluePrints/BP_MySaveGame.BP_MySaveGame_C"))
  (Variables|/Game/Project/BluePrints/BP_MySaveGame.BP_MySaveGame_C|SetEventState _returnvalue (Variables|Default|GetEventStatus))
  (Variables|/Game/Project/BluePrints/BP_MySaveGame.BP_MySaveGame_C|SetKeyStatus _returnvalue (Variables|Default|GetKeyStatus))
  (Variables|/Game/Project/BluePrints/BP_MySaveGame.BP_MySaveGame_C|SetPlayerSaveTransform _returnvalue (Variables|Default|GetPlayerTransform))
  (Variables|/Game/Project/BluePrints/BP_MySaveGame.BP_MySaveGame_C|SetPlayerItemNameList _returnvalue (Variables|Default|GetPlayerItemNameList))
  (SaveGame|SaveGametoSlot _returnvalue "MySaveGame"))

(event Custom|ImportSaveData
  (bind _returnvalue (SaveGame|LoadGamefromSlot "MySaveGame"))
  (bind _asbp_my_save_game (Utilities|Casting|CastToBP_MySaveGame _returnvalue))
  (Variables|Default|SetEventStatus (Variables|/Game/Project/BluePrints/BP_MySaveGame.BP_MySaveGame_C|GetEventState _asbp_my_save_game))
  (Variables|Default|SetKeyStatus (Variables|/Game/Project/BluePrints/BP_MySaveGame.BP_MySaveGame_C|GetKeyStatus _asbp_my_save_game))
  (Variables|Default|SetPlayerTransform (Variables|/Game/Project/BluePrints/BP_MySaveGame.BP_MySaveGame_C|GetPlayerSaveTransform _asbp_my_save_game))
  (Variables|Default|SetPlayerItemNameList (Variables|/Game/Project/BluePrints/BP_MySaveGame.BP_MySaveGame_C|GetPlayerItemNameList _asbp_my_save_game)))

(event Custom|DeleteSaveData
  (Utilities|Map|Clear (Variables|Default|GetEventStatus))
  (Utilities|Map|Clear (Variables|Default|GetKeyStatus))
  (Variables|Default|SetPlayerTransform "")
  (Utilities|Map|Clear (Variables|Default|GetPlayerItemNameList))
  (SaveGame|DeleteGameinSlot "MySaveGame")
  (Development|PrintString "DeleteSaveData"))

(event EventInit
  (CallFunction|ImportSaveData))

(fn SaveEventStatus
  (params (Event%20Name :type Name) (Status :type EN_EventStatus%20Enum :default "NewEnumerator0"))
  (Utilities|Map|Add (Variables|Default|GetEventStatus) Event%20Name Status)
  (CallFunction|ExportSaveData))

(fn GetEventStatus
  (params (Event%20Status :type Name))
  (bind _eventstatus (Variables|Default|GetEventStatus))
  (bind (_value _returnvalue) (Utilities|Map|Find _eventstatus Event%20Status))
  (if _returnvalue
    (return _value)
    (else
      (return "NewEnumerator0"))))

(fn SaveKeyStatus
  (params (Key%20Name :type Name) (Status :type EN_KeyStatus%20Enum :default "NewEnumerator3"))
  (Utilities|Map|Add (Variables|Default|GetKeyStatus) Key%20Name Status)
  (CallFunction|ExportSaveData))

(fn GetKeyStatus
  (params (Key%20Name :type Name))
  (bind _keystatus (Variables|Default|GetKeyStatus))
  (bind (_value _returnvalue) (Utilities|Map|Find _keystatus Key%20Name))
  (if _returnvalue
    (return _value)
    (else
      (return "NewEnumerator3"))))

(fn SavePlayerTransform
  (params (PlayerTransform :type Transform))
  (Variables|Default|SetPlayerTransform PlayerTransform)
  (CallFunction|ExportSaveData))

(fn LoadPlayerTransform
  (return (Variables|Default|GetPlayerTransform)))

(fn SavePlayerItemNameList
  (params (ItemNameList :type Map%20of%20Names%20to%20Integers))
  (Variables|Default|SetPlayerItemNameList ItemNameList)
  (CallFunction|ExportSaveData))

(fn GetPlayerItemNameList
  (return (Variables|Default|GetPlayerItemNameList)))