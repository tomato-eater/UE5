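; Character Blueprint that handles health, damage and ragdoll death.
; The construction script fills current HP to max, and AnyDamage subtracts from it, broadcasts the HP change and calls UpDataGauge, which is empty here.
; At zero or below, a DoOnce guard triggers CharaDeadEvent, which disables input, switches the mesh to physics-simulated ragdoll and sets a short lifespan so the actor is removed.
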(event EventBeginPlay)

(event Collision|EventActorBeginOverlap
  (params (OtherActor :type Actor%20Object%20Reference)))

(event Game|Damage|EventAnyDamage
  (params (Damage :type Float%20%28single-precision%29) (DamageType :type Damage%20Type%20Object%20Reference) (InstigatedBy :type Controller%20Object%20Reference) (DamageCauser :type Actor%20Object%20Reference))
  (bind _output_get (Variables|Default|SetCurrentHP (- (Variables|Default|GetCurrentHP) Damage)))
  (Default|CallOnCharaHpChanged _output_get (Variables|Default|GetMaxHP))
  (CallFunction|UpDataGauge)
  (if (<= _output_get 0.0)
    (Utilities|FlowControl|DoOnce false
      (:Completed
        (CallFunction|CharaDeadEvent)))))

(event EventTick
  (params (DeltaSeconds :type Float%20%28single-precision%29)))

(fn ConstructionScript
  (Variables|Default|SetCurrentHP (Variables|Default|GetMaxHP)))

(fn CharaDeadEvent
  (bind _mesh (Variables|Character|GetMesh))
  (Input|DisableInput 0)
  (Collision|SetCollisionProfileName _mesh "Ragdoll" true :!class /Script/Engine.PrimitiveComponent)
  (Physics|SetSimulatePhysics _mesh true)
  (Actor|SetLifeSpan 3.0))

(fn UpDataGauge)