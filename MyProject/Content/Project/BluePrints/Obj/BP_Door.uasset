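; Door Blueprint that swings open when a Player-tagged component overlaps its collision box, with optional key and switch gating.
; Doors without a key or switch flag open directly; others require a Got key status in the game instance, which resets to Default on use.
; The Open timeline drives mesh yaw and disables the trigger collision.
; On completion, SetEventFinished calls the parent, clears the switch flag and snaps the door to 90 degrees.
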(event OnComponentBeginOverlap(CollisionBox)
  (params (OverlappedComponent :type Primitive%20Component%20Object%20Reference) (OtherActor :type Actor%20Object%20Reference) (OtherComp :type Primitive%20Component%20Object%20Reference) (OtherBodyIndex :type Integer) (bFromSweep :type Boolean) (SweepResult :type Hit%20Result%20Structure%20%28by%20ref%29))
  (bind _keyname (Variables|Default|GetKeyName))
  (bind _mygameinstance (Variables|Default|GetMyGameInstance))
  (if (Components|ComponentHasTag OtherComp "Player")
    (if (and (== _keyname "") (not (Variables|Default|GetSwitchDoor)))
      _
      (else
        (switch Utilities|FlowControl|Switch|SwitchonEN_KeyStatus (Default|GetKeyStatus _mygameinstance _keyname)
          (:NewEnumerator4
            (Default|SaveKeyStatus _mygameinstance _keyname "NewEnumerator3")))))
    (CallFunction|OpenDoor)))

(event Custom|OpenDoor
  (Variables|Default|SetSwitchDoor false)
  (bind _openz (Timeline|Open Play)
    (:Update
      (Transformation|SetRelativeRotation (Variables|Default|GetSTM_Door) (Math|Rotator|MakeRotator 0.0 0.0 _openz) false false)
      (Collision|SetCollisionEnabled (Variables|Default|GetCollisionBox) "NoCollision"))
    (:Finished
      (CallFunction|SetEventFinished))))

(event EventBeginPlay
  (|CallParentFunction))

(fn ConstructionScript)

(fn SetEventFinished
  (|CallParentFunction)
  (Variables|Default|SetSwitchDoor false)
  (Transformation|SetRelativeRotation (Variables|Default|GetSTM_Door) "0.000000,90.000000,0.000000" false false)
  (Collision|SetCollisionEnabled (Variables|Default|GetCollisionBox) "NoCollision"))