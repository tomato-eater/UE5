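; BP_Key is a key pickup that the player collects by walking into its sphere.
; On overlap with a component tagged Player, it notifies the player through ACOverlapPlayer using its KeyName and saves that key's status in the game instance.
; It then finishes its event by calling the parent's SetEventFinished and destroying itself.
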(event OnComponentBeginOverlap(Sphere)
  (params (OverlappedComponent :type Primitive%20Component%20Object%20Reference) (OtherActor :type Actor%20Object%20Reference) (OtherComp :type Primitive%20Component%20Object%20Reference) (OtherBodyIndex :type Integer) (bFromSweep :type Boolean) (SweepResult :type Hit%20Result%20Structure%20%28by%20ref%29))
  (bind _keyname (Variables|Default|GetKeyName))
  (if (Components|ComponentHasTag OtherComp "Player")
    (Default|NotifytoPlayer (Variables|Default|GetAC_OverlapPlayer) OtherActor _keyname)
    (Default|SaveKeyStatus (Variables|Default|GetMyGameInstance) _keyname "NewEnumerator4")
    (CallFunction|SetEventFinished)))

(event EventBeginPlay
  (if true
    (|CallParentFunction)))

(fn ConstructionScript)

(fn SetEventFinished
  (|CallParentFunction)
  (Actor|DestroyActor))