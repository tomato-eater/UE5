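; BP_Lever is an interactable lever that opens a linked door when shifted.
; ShiftLevel plays a timeline that pitches the lever mesh along its LeverY curve and turns off the Box collision during the motion.
; When the timeline finishes, it calls OpenDoor on TargetDoor if valid and then marks the event finished through the parent class's SetEventFinished.
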(event Custom|ShiftLevel
  (bind _lever_y (Timeline|タイムライン Play)
    (:Update
      (Transformation|SetRelativeRotation (Variables|Default|GetSTM_Lever) (Math|Rotator|MakeRotator 0.0 _lever_y 0.0) false false)
      (Collision|SetCollisionEnabled (Variables|Default|GetBox) "NoCollision"))
    (:Finished
      (bind _targetdoor (Variables|Default|GetTargetDoor)
        (:then
          (Default|OpenDoor _targetdoor)
          (CallFunction|SetEventFinished))
        (:else)))))

(fn ConstructionScript
  (|CallParentFunction))

(fn SetEventFinished
  (|CallParentFunction))