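; BP_SwitchButton is a switch button that opens a linked door when a component tagged "Player" overlaps its Box.
; The SwitchON timeline animates the STMButton mesh on Z, then opens TargetDoor and marks MoveBox's event finished, when each is valid.
; It then calls its own SetEventFinished, which extends the parent's version by setting the mesh to relative origin and disabling Box collision.
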(event OnComponentBeginOverlap(Box)
  (params (OverlappedComponent :type Primitive%20Component%20Object%20Reference) (OtherActor :type Actor%20Object%20Reference) (OtherComp :type Primitive%20Component%20Object%20Reference) (OtherBodyIndex :type Integer) (bFromSweep :type Boolean) (SweepResult :type Hit%20Result%20Structure%20%28by%20ref%29))
  (bind _movebox (Variables|Default|GetMoveBox))
  (bind _targetdoor (Variables|Default|GetTargetDoor))
  (if (Components|ComponentHasTag OtherComp "Player")
    (bind _buttonz (Timeline|SwitchON Play)
      (:Update
        (Transformation|SetRelativeLocation (Variables|Default|GetSTM_Button) (Math|Vector|MakeVector 0.0 0.0 _buttonz) false false))
      (:Finished
        (Utilities|FlowControl|Sequence
          (:then_0
            (if (Utilities|IsValid _targetdoor)
              (Default|OpenDoor _targetdoor)
              (CallFunction|SetEventFinished)))
          (:then_1
            (if (Utilities|IsValid _movebox)
              (CallFunction|SetEventFinished _movebox)))
          (:then_2
            (CallFunction|SetEventFinished)))))))

(event EventBeginPlay
  (|CallParentFunction))

(fn ConstructionScript)

(fn SetEventFinished
  (|CallParentFunction)
  (Transformation|SetRelativeLocation (Variables|Default|GetSTM_Button) "0, 0, 0" false false)
  (Collision|SetCollisionEnabled (Variables|Default|GetBox) "NoCollision"))