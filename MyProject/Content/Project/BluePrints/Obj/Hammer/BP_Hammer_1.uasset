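; BP_Hammer_1 is a swinging hammer obstacle that knocks the player character away on contact.
; A timeline, triggered from Tick and restarted through ReRotato when it finishes, drives the Hammer's relative pitch in a continuous loop.
; Box overlap with a BP_TestChar launches it along the normalized direction away from the actor, scaled strongly on world X, slightly on Z and zeroed on Y.
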(event OnComponentBeginOverlap(Box)
  (params (OverlappedComponent :type Primitive%20Component%20Object%20Reference) (OtherActor :type Actor%20Object%20Reference) (OtherComp :type Primitive%20Component%20Object%20Reference) (OtherBodyIndex :type Integer) (bFromSweep :type Boolean) (SweepResult :type Hit%20Result%20Structure%20%28by%20ref%29))
  (bind _asbp_test_char (Utilities|Casting|CastToBP_TestChar OtherActor))
  (Character|LaunchCharacter _asbp_test_char (* (Math|Vector|Normalize (- (Transformation|GetActorLocation _asbp_test_char) (Transformation|GetActorLocation))) "10000.000000,0.000000,5.000000") false false))

(event Custom|ReRotato
  (bind _rothamm (Timeline|タイムライン PlayFromStart)
    (:Update
      (Transformation|SetRelativeRotation (Variables|Default|GetHammer) (Math|Rotator|MakeRotator 0.0 _rothamm 0.0) false false))
    (:Finished
      (CallFunction|ReRotato))))

(event EventBeginPlay)

(event Collision|EventActorBeginOverlap
  (params (OtherActor :type Actor%20Object%20Reference)))

(event EventTick
  (params (DeltaSeconds :type Float%20%28single-precision%29))
  (bind _rothamm (Timeline|タイムライン Play)
    (:Update
      (Transformation|SetRelativeRotation (Variables|Default|GetHammer) (Math|Rotator|MakeRotator 0.0 _rothamm 0.0) false false))
    (:Finished
      (CallFunction|ReRotato))))

(fn ConstructionScript)